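; BP_MasterInteract is a master actor for interactable objects that tells the player when it comes within or leaves interaction range.
; Its InteractRangeSphere overlap events cast the other actor to BP_Player and add or remove this object as an interaction overlap.
; The construction script sizes the sphere from the InteractRangeSphereRadius variable.
; IsInteractable returns false here, serving as a default answer.
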(event OnComponentBeginOverlap(InteractRangeSphere)
  (params (OverlappedComponent :type Primitive%20Component%20Object%20Reference) (OtherActor :type Actor%20Object%20Reference) (OtherComp :type Primitive%20Component%20Object%20Reference) (OtherBodyIndex :type Integer) (bFromSweep :type Boolean) (SweepResult :type Hit%20Result%20Structure%20%28by%20ref%29))
  (bind _asbp_player (Utilities|Casting|CastToBP_Player OtherActor))
  (Default|AddInteractionOverlap _asbp_player self))

(event OnComponentEndOverlap(InteractRangeSphere)
  (params (OverlappedComponent :type Primitive%20Component%20Object%20Reference) (OtherActor :type Actor%20Object%20Reference) (OtherComp :type Primitive%20Component%20Object%20Reference) (OtherBodyIndex :type Integer))
  (bind _asbp_player (Utilities|Casting|CastToBP_Player OtherActor))
  (Default|RemoveInteractionOverlap _asbp_player self))

(fn ConstructionScript
  (Components|Sphere|SetSphereRadius (Variables|Default|GetInteractRangeSphere) (Variables|Default|GetInteractRangeSphereRadius) true))

(fn IsInteractable
  (return false))