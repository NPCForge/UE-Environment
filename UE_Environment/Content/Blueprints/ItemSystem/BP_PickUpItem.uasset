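; BP_PickUpItem is a pickup item actor whose appearance is driven by an item data table.
; Its construction script looks up the row referenced by the item's slot, then copies the row's name and mesh.
; The static mesh's relative scale is set to the actor scale multiplied by the row's rescale factor.
; OnInteract is an empty stub, so no pickup logic runs in this graph.
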(event EventBeginPlay
  (|CallParentFunction) ; This node is disabled and will not be called.\nDrag off pins to build functionality.
)

(event Collision|EventActorBeginOverlap
  (params (OtherActor :type Actor%20Object%20Reference))
  (|CallParentFunction OtherActor) ; This node is disabled and will not be called.\nDrag off pins to build functionality.
)

(event EventTick
  (params (DeltaSeconds :type Float%20%28single-precision%29))
  (|CallParentFunction DeltaSeconds) ; This node is disabled and will not be called.\nDrag off pins to build functionality.
)

(event EventOnInteract
  (params (Interacting%20Character :type Character%20Object%20Reference)))

(fn ConstructionScript
  (bind _item (Variables|Default|GetItem))
  (|CallParentFunction)
  (bind _returnvalue (Utilities|GetDataTableRow (.datatable (.slot _item)) (.rowname (.slot _item)))
    (:then
      (Variables|Default|SetName (.Name (Utilities|Struct|BreakS_Item _returnvalue)))
      (Components|StaticMesh|SetStaticMesh (Variables|Default|GetStaticMesh) (.Mesh (Utilities|Struct|BreakS_Item _returnvalue)))
      (Transformation|SetRelativeScale3D (Variables|Default|GetStaticMesh) (* (Transformation|GetActorScale3D) (.MeshRescale (Utilities|Struct|BreakS_Item _returnvalue)))))))